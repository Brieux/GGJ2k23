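; Spline road actor that lays spline mesh segments along its spline in the Construction Script, with no active runtime logic.
; It divides the spline length by Length and adds one non-colliding mesh per step, using positions and size-clamped tangents sampled by distance.
; Each step also runs a debug-drawn downward trace from the spline point at the loop index, but the hit does not affect placement.
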(fn `UserConstructionScript`
  (bind _spline (`self.Spline`))
  (bind _length (`self.length`))
  (for _index (range (`KismetMathLibrary.FTrunc` (/ (`SplineComponent.GetSplineLength` (`self.Spline`)) (`self.length`))))
    (bind _returnvalue (`SplineComponent.GetLocationAtSplinePoint` (`self.Spline`) _index "Local"))
    (bind _outhit (`KismetSystemLibrary.LineTraceSingle` :`Start` _returnvalue :`End` (`KismetMathLibrary.MakeVector` (.x _returnvalue) (.y _returnvalue) (- (.z _returnvalue) 1000.0)) :`TraceChannel` "TraceTypeQuery1" :`DrawDebugType` "ForDuration"))
    (set `self.Out Hit Location` (`.ImpactPoint` (`GameplayStatics.BreakHitResult` _outhit)))
    (bind _returnvalue_2 (`AddComponent|NODE_AddSplineMeshComponent-1` :`RelativeTransform` (`KismetMathLibrary.MakeTransform` (0.0 0.0 0.0) (struct))))
    (`SplineMeshComponent.SetForwardAxis` _returnvalue_2 "X" true)
    (`PrimitiveComponent.SetCollisionEnabled` _returnvalue_2 "NoCollision")
    (bind _returnvalue_3 (* _length _index))
    (bind _returnvalue_4 (* _length (+ _index 1)))
    (`SplineMeshComponent.SetStartAndEnd` _returnvalue_2 (`SplineComponent.GetLocationAtDistanceAlongSpline` _spline _returnvalue_3 "Local") (`KismetMathLibrary.ClampVectorSize` (`SplineComponent.GetTangentAtDistanceAlongSpline` _spline _returnvalue_3 "Local") 0.0 1.0) (`SplineComponent.GetLocationAtDistanceAlongSpline` _spline _returnvalue_4 "Local") (`KismetMathLibrary.ClampVectorSize` (`SplineComponent.GetTangentAtDistanceAlongSpline` _spline _returnvalue_4 "Local") 0.0 1.0) true)))