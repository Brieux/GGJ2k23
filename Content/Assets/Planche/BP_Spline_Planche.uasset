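; BP_Spline_Planche is a spline-based placement Blueprint, apparently for planks, that repeats a static mesh along a path.
; The construction script divides the spline length by the Distance spacing and loops over the resulting count, adding a mesh component at each step.
; Each component takes the spline's local location and rotation at that distance, keeps unit scale and uses the Mesh variable.
; The event graph contains no active logic.
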(fn `UserConstructionScript`
  (bind _spline (`self.Spline`))
  (for _index (range (+ (`.ReturnValue` (`KismetMathLibrary.FMod` (`SplineComponent.GetSplineLength` (`self.Spline`)) (`self.Distance`))) 1))
    (bind _returnvalue (* _index (`self.Distance`)))
    (bind _returnvalue_2 (`AddComponent|NODE_AddStaticMeshComponent-0` :`RelativeTransform` (`KismetMathLibrary.MakeTransform` (`SplineComponent.GetLocationAtDistanceAlongSpline` _spline _returnvalue "Local") (`SplineComponent.GetRotationAtDistanceAlongSpline` _spline _returnvalue "Local"))))
    (`StaticMeshComponent.SetStaticMesh` _returnvalue_2 (`self.Mesh`))))