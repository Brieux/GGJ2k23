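; Player controller that routes Enhanced Input to the third-person character.
; On BeginPlay it adds the default mapping context, then casts the controlled pawn to BP_ThirdPersonCharacter and caches it.
; Move, Look and Jump input actions forward their values and press/release events to that cached character's functions.
; The reference is set only at BeginPlay, with no refresh on possession changes.
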(event `self.ReceiveBeginPlay`
  (bind _returnvalue (pcsubsystem `EnhancedInputLocalPlayerSubsystem` self))
  (`/Engine/EditorBlueprintResources/StandardMacros.IsValid` _returnvalue
    (:`Is Valid`
      (`EnhancedInputSubsystemInterface.AddMappingContext` _returnvalue "/Game/ThirdPerson/Input/IMC_Default.IMC_Default" 0 (struct))
      (bind _asbp_third_person_character (cast `/Game/ThirdPerson/Blueprints/BP_ThirdPersonCharacter` (`self.K2_GetPawn`)))
      (set `self.As BP Third Person Character` _asbp_third_person_character))))

(event `EnhancedInput|/Game/ThirdPerson/Input/Actions/IA_Move`
  (params (ActionValue :type "Vector2D Structure") (ElapsedSeconds :type "Float (double-precision)") (TriggeredSeconds :type "Float (double-precision)") (InputAction :type "InputAction Object Reference" :default "/Game/ThirdPerson/Input/Actions/IA_Move.IA_Move"))
  (:`Triggered`
    (`/Game/ThirdPerson/Blueprints/BP_ThirdPersonCharacter.Move` (`self.As BP Third Person Character`) ActionValue_X ActionValue_Y)))

(event `EnhancedInput|/Game/ThirdPerson/Input/Actions/IA_Look`
  (params (ActionValue :type "Vector2D Structure") (ElapsedSeconds :type "Float (double-precision)") (TriggeredSeconds :type "Float (double-precision)") (InputAction :type "InputAction Object Reference" :default "/Game/ThirdPerson/Input/Actions/IA_Look.IA_Look"))
  (:`Triggered`
    (`/Game/ThirdPerson/Blueprints/BP_ThirdPersonCharacter.Look` (`self.As BP Third Person Character`) ActionValue_X ActionValue_Y)))

(event `EnhancedInput|/Game/ThirdPerson/Input/Actions/IA_Jump`
  (params (ActionValue :type Boolean) (ElapsedSeconds :type "Float (double-precision)") (TriggeredSeconds :type "Float (double-precision)") (InputAction :type "InputAction Object Reference" :default "/Game/ThirdPerson/Input/Actions/IA_Jump.IA_Jump"))
  (bind _as_bp_third_person_character (`self.As BP Third Person Character`))
  (:`Started`
    (`/Game/ThirdPerson/Blueprints/BP_ThirdPersonCharacter.Jumping` _as_bp_third_person_character))
  (:`Completed`
    (`/Game/ThirdPerson/Blueprints/BP_ThirdPersonCharacter.StopJump` _as_bp_third_person_character)))

(fn `UserConstructionScript`)